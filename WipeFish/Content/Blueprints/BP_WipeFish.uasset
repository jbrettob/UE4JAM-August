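; BP_WipeFish is a physics-driven hover vehicle with four corner hover components, propelled by forward force and steered by yaw torque that inverts when not moving forward.
; Input comes from axes, or from latching WASD toggles when JayceRemote is set.
; Each tick, a velocity-predicted downward trace aligns pitch and roll to the surface normal, easing toward world up on a miss.
; Spring-arm camera lag interpolates between limits by speed band.
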(event `self.ReceiveBeginPlay`
  (`/Game/Blueprints/HoverComponent.InitComponent` (`self.HoverComponent_RL`) (`self.Mesh`))
  (`/Game/Blueprints/HoverComponent.InitComponent` (`self.HoverComponent_FR`) (`self.Mesh`))
  (`/Game/Blueprints/HoverComponent.InitComponent` (`self.HoverComponent_RR`) (`self.Mesh`))
  (`/Game/Blueprints/HoverComponent.InitComponent` (`self.HoverComponent_FL`) (`self.Mesh`))
  (`/Game/Blueprints/HoverComponent.SetDebug` (`self.HoverComponent_RL`) (`self.bDebug`))
  (`/Game/Blueprints/HoverComponent.SetDebug` (`self.HoverComponent_FR`) (`self.bDebug`))
  (`/Game/Blueprints/HoverComponent.SetDebug` (`self.HoverComponent_RR`) (`self.bDebug`))
  (`/Game/Blueprints/HoverComponent.SetDebug` (`self.HoverComponent_FL`) (`self.bDebug`)))

(event `self.ReceiveTick`
  (params (DeltaSeconds :type "Float (single-precision)"))
  (`self.UpdateCameraLag`)
  (`self.UpdateSurfaceNormal`))

(event `InputAxis|MoveForward`
  (params (AxisValue :type "Float (single-precision)"))
  (`self.UpdateMoveForward` (`KismetMathLibrary.SelectFloat` (select `bool` (`self.bWPressed`) :`false` (`KismetMathLibrary.SelectFloat` -1.0 0.0 (`self.bSPressed`)) :`true` 1.0) AxisValue (`self.JayceRemote`))))

(event `InputAxis|MoveRight`
  (params (AxisValue :type "Float (single-precision)"))
  (`self.UpdateMoveRight` (`KismetMathLibrary.SelectFloat` (select `bool` (`self.bDPressed`) :`false` (select `bool` (`self.bAPressed`) :`true` -1.0 :!type "Float (single-precision)") :`true` 1.0) AxisValue (`self.JayceRemote`))))

(event `Key|W`
  (params (Key :type "Key Structure" :default "AnyKey"))
  (:`Pressed`
    (set `self.bWPressed` (not (`self.bWPressed`)))
    (set `self.bSPressed` false)))

(event `Key|S`
  (params (Key :type "Key Structure" :default "AnyKey"))
  (:`Pressed`
    (set `self.bSPressed` (not (`self.bSPressed`)))
    (set `self.bWPressed` false)))

(event `Key|A`
  (params (Key :type "Key Structure" :default "AnyKey"))
  (:`Pressed`
    (set `self.bAPressed` (not (`self.bAPressed`)))
    (set `self.bDPressed` false)))

(event `Key|D`
  (params (Key :type "Key Structure" :default "AnyKey"))
  (:`Pressed`
    (set `self.bDPressed` (not (`self.bDPressed`)))
    (set `self.bAPressed` false)))

(fn `GetPredictedLocation`
  (returns (Location :type "Vector Structure"))
  (bind _mesh (`self.Mesh`))
  (return (+ (`SceneComponent.K2_GetComponentLocation` _mesh) (* (`SceneComponent.GetForwardVector` _mesh) (* (`KismetMathLibrary.VSize` (`SceneComponent.GetComponentVelocity` _mesh)) 0.5)))))

(fn `UpdateCameraLag`
  (bind _bdebug (`self.bDebug`))
  (bind _returnvalue (`PrimitiveComponent.GetPhysicsLinearVelocity` (`self.Mesh`) "None"))
  (bind _returnvalue_2 (`KismetMathLibrary.VSize` _returnvalue))
  (`KismetSystemLibrary.PrintText` (`|FormatText` "Velocity: {Velocity}" (`KismetTextLibrary.Conv_StringToText` (`KismetStringLibrary.Conv_DoubleToString` _returnvalue_2))) _bdebug _bdebug)
  (if (and (>= _returnvalue_2 1500.0) (< _returnvalue_2 2250.0))
    (set `SpringArmComponent.CameraLagSpeed` (`KismetMathLibrary.FInterpTo` (`SpringArmComponent.CameraLagSpeed` (`self.SpringArm`)) (`self.CameraLagMin`) (`GameplayStatics.GetWorldDeltaSeconds`) 0.8) (`self.SpringArm`))
    (else
      (set `SpringArmComponent.CameraLagSpeed` (`KismetMathLibrary.FInterpTo` (`SpringArmComponent.CameraLagSpeed` (`self.SpringArm`)) (`self.CameraLagMax`) (`GameplayStatics.GetWorldDeltaSeconds`) 0.4) (`self.SpringArm`))))
  (return))

(fn `UpdateMoveForward`
  (params (AxisSpeed :type "Float (double-precision)"))
  (`PrimitiveComponent.AddForce` (`self.Mesh`) (* (`SceneComponent.GetForwardVector` (`self.Mesh`)) (* AxisSpeed (`self.MovementSpeed`))) "None" false)
  (return))

(fn `UpdateMoveRight`
  (params (AxisValue :type "Float (double-precision)"))
  (bind _returnvalue (`PrimitiveComponent.GetPhysicsLinearVelocity` (`self.Mesh`) "None"))
  (`PrimitiveComponent.AddTorque` (`self.Mesh`) (`KismetMathLibrary.MakeVector` 0.0 0.0 (* (* AxisValue (`self.RotationSpeed`)) (`KismetMathLibrary.SelectFloat` 1.0 -1.0 (> (`KismetMathLibrary.Dot_VectorVector` _returnvalue (`SceneComponent.GetForwardVector` (`self.Mesh`))) 0.0)))) "None" false)
  (return))

(fn `UpdateSurfaceNormal`
  (bind _location (`self.GetPredictedLocation`))
  (bind _returnvalue (`KismetMathLibrary.MakeVector` 0.0 0.0 1.0))
  (bind _mesh (`self.Mesh`))
  (bind _mesh_2 (`self.Mesh`))
  (bind _returnvalue_2 (`SceneComponent.K2_GetComponentRotation` _mesh_2))
  (bind _returnvalue_3 (`SceneComponent.K2_GetComponentRotation` _mesh))
  (bind (_outhit _returnvalue_4) (`KismetSystemLibrary.LineTraceSingle` _location (+ _location (* (`SceneComponent.GetUpVector` (`self.Mesh`)) -1000)) "TraceTypeQuery1" true))
  (if _returnvalue_4
    (bind (_bblockinghit _binitialoverlap _time _location_2 _impactpoint _normal _impactnormal) (`GameplayStatics.BreakHitResult` _outhit))
    ;[1 1 1] // Orientate towards sufrace norma
    (`SceneComponent.K2_SetWorldRotation` (`self.Mesh`) (`KismetMathLibrary.RInterpTo` _returnvalue_3 (`KismetMathLibrary.MakeRotator` (.roll (`KismetMathLibrary.MakeRotFromXZ` (`SceneComponent.GetForwardVector` _mesh) _impactnormal)) (.pitch (`KismetMathLibrary.MakeRotFromYZ` (`SceneComponent.GetRightVector` _mesh) _impactnormal)) (.yaw _returnvalue_3)) (`GameplayStatics.GetWorldDeltaSeconds`) 10.0) false false)
    (else
      (`SceneComponent.K2_SetWorldRotation` (`self.Mesh`) (`KismetMathLibrary.RInterpTo` _returnvalue_2 (`KismetMathLibrary.MakeRotator` (.roll (`KismetMathLibrary.MakeRotFromXZ` (`SceneComponent.GetForwardVector` _mesh_2) _returnvalue)) (.pitch (`KismetMathLibrary.MakeRotFromYZ` (`SceneComponent.GetRightVector` _mesh_2) _returnvalue)) (.yaw _returnvalue_2)) (`GameplayStatics.GetWorldDeltaSeconds`) 1.0) false false))))

(fn `UserConstructionScript`
  (`parent.UserConstructionScript`))