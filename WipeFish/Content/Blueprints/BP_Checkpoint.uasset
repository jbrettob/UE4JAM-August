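; BP_Checkpoint is a checkpoint actor that runs a timer and shows the elapsed time on a text render.
; Tick accumulates time through a gate, which Stop closes once via a DoOnce and Reset reopens after zeroing the time and re-arming the DoOnce.
; The construction script forces unit actor scale, then applies trigger box scale and text position from variables.
; GetTimeInSeconds returns the time as a formatted string.
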(event `self.ReceiveTick`
  (params (DeltaSeconds :type "Float (single-precision)"))
  (`/Engine/EditorBlueprintResources/StandardMacros.Gate` false :!label _label
    (:`Exit`
      (set `self.TimeInSeconds` (+ DeltaSeconds (`self.TimeInSeconds`)))
      (`TextRenderComponent.K2_SetText` (`self.TextRender`) (`KismetTextLibrary.Conv_StringToText` (`KismetStringLibrary.TimeSecondsToString` (`self.TimeInSeconds`)))))))

(event `Stop`
  (`/Engine/EditorBlueprintResources/StandardMacros.DoOnce` false :!label _label_2
    (:`Completed`
      (`|ExecutionSequence`
        (:`then_0`
          (goto _label :!via `Close`))))))

(event `Reset`
  (`|ExecutionSequence`
    (:`then_0`
      (goto _label_2 :!via `Reset`))
    (:`then_1`
      (set `self.TimeInSeconds` 0.0)
      (goto _label :!via `Open`))))

(fn `GetTimeInSeconds`
  (returns (TimeInSeconds :type String))
  (return (`KismetStringLibrary.TimeSecondsToString` (`self.TimeInSeconds`))))

(fn `UserConstructionScript`
  (`self.SetActorScale3D` (1.0 1.0 1.0))
  (`SceneComponent.SetWorldScale3D` (`self.TriggerBox`) (`self.TriggerBoxScale`))
  (`SceneComponent.K2_SetRelativeLocation` (`self.TextRender`) (`self.TextLocation`) false false))