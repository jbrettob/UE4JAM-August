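; Road generator Blueprint that builds a randomized spline road with obstacles in its construction script.
; It rebuilds the spline with points stepped along negative Y and random, unseeded X offsets, so the layout changes whenever construction reruns.
; Each point spawns a spline mesh toward the next, divided by MeshScaleVec, plus a raised, scaled-up static mesh obstacle at random X offset.
; An editable-spline variant is disconnected, and the event graph is empty.
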(fn `UserConstructionScript`
  (bind _spline (`self.Spline`))
  (bind _spline_2 (`self.Spline`))
  (bind _meshscalevec (`self.MeshScaleVec`))
  ;[1 1 1] Create spline road
  (`SplineComponent.ClearSplinePoints` _spline_2)
  (for _index (range (+ (`self.Sections`) 1))
    (`SplineComponent.AddSplinePoint` (`self.Spline`) (+ (`KismetMathLibrary.MakeVector` (`KismetMathLibrary.RandomFloatInRange` -1000.0 1000.0) (* _index -5000.0)) (`SplineComponent.GetLocationAndTangentAtSplinePoint` _spline_2 0 "Local")) "Local"))
  (for _index_2 (range (+ (`SplineComponent.GetNumberOfSplinePoints` (`self.Spline`)) 1))
    (bind _returnvalue (`AddComponent|SplineMeshComponent_1`))
    (bind (_location _tangent) (`SplineComponent.GetLocationAndTangentAtSplinePoint` _spline _index_2 "Local"))
    (bind (_location_2 _tangent_2) (`SplineComponent.GetLocationAndTangentAtSplinePoint` _spline (+ _index_2 1) "Local"))
    (`SplineMeshComponent.SetStartAndEnd` _returnvalue (/ _location _meshscalevec) (/ _tangent _meshscalevec) (/ _location_2 _meshscalevec) (/ _tangent_2 _meshscalevec) true)
    ;[1 1 1] Create obstacles
    (`AddComponent|StaticMeshComponent_5` :`RelativeTransform` (`KismetMathLibrary.MakeTransform` (+ _location (`KismetMathLibrary.MakeVector` (`KismetMathLibrary.RandomFloatInRange` -1000.0 1000.0) 0.0 1000.0)) (struct) (5.0 5.0 5.0)))))