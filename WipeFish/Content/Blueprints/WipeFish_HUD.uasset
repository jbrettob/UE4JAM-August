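; WipeFish_HUD is a HUD Blueprint that draws a time readout in seconds near the top-left of the screen.
; On BeginPlay it searches all BP_Checkpoint actors for the one with display name "BP_Checkpoint9" and caches it as FinalCheckpoint.
; While that reference is valid, DrawHUD shows the checkpoint's GetTimeInSeconds value, so the readout depends on that hardcoded actor name.
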(event `self.ReceiveDrawHUD`
  (params (SizeX :type Integer) (SizeY :type Integer))
  (`/Engine/EditorBlueprintResources/StandardMacros.IsValid` (`self.Final Checkpoint`)
    (:`Is Valid`
      (`self.DrawText` (`KismetStringLibrary.Concat_StrStr` "Time: " (`/Game/Blueprints/BP_Checkpoint.GetTimeInSeconds` (`self.Final Checkpoint`))) (struct :`G` 1.0 :`B` 0.953681 :`A` 1.0) 30.0 30.0 "/Engine/EngineFonts/Roboto.Roboto" 1.0 true))))

(event `self.ReceiveBeginPlay`
  (bind _outactors (`GameplayStatics.GetAllActorsOfClass` "/Game/Blueprints/BP_Checkpoint.BP_Checkpoint_C"))
  (for _array_element _outactors
    (if (`KismetStringLibrary.EqualEqual_StrStr` (`KismetSystemLibrary.GetDisplayName` _array_element) "BP_Checkpoint9")
      (set `self.Final Checkpoint` _array_element)
      (break))))

(fn `UserConstructionScript`)