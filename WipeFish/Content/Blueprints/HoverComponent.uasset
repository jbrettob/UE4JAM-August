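; HoverComponent is a hover thruster that pushes a physics-simulated static mesh away from the surface beneath it.
; InitComponent stores the mesh, turns on physics and enables tick.
; Each tick traces along the component's negative up vector and, on a hit, applies force at its own location along the impact normal, fading linearly to zero at trace length.
; Hits also set the mesh's damping; SetDebug toggles trace drawing.
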(event `InitComponent`
  (params (StaticMeshComponent :type "PrimitiveComponent Object Reference"))
  (bind _output_get (set `self.ParentComponent` StaticMeshComponent))
  (`PrimitiveComponent.SetSimulatePhysics` _output_get true)
  (`self.SetComponentTickEnabled` true))

(event `self.ReceiveTick`
  (params (DeltaSeconds :type "Float (single-precision)"))
  (`/Engine/EditorBlueprintResources/StandardMacros.IsValid` (`self.ParentComponent`)
    (:`Is Valid`
      (bind (_outhit _returnvalue) (`KismetSystemLibrary.LineTraceSingle` :`Start` (`self.K2_GetComponentLocation`) :`End` (+ (`self.K2_GetComponentLocation`) (* (`self.GetUpVector`) (* (`self.TraceLength`) -1.0))) :`TraceChannel` "TraceTypeQuery1" :`bTraceComplex` true :`DrawDebugType` (select `bool` (`self.bDebug`) :`true` "ForDuration" :!type "EDrawDebugTrace Enum")))
      (if _returnvalue
        (bind (_bblockinghit _binitialoverlap _time _location _impactpoint _normal _impactnormal) (`GameplayStatics.BreakHitResult` _outhit))
        (`PrimitiveComponent.AddForceAtLocation` (`self.ParentComponent`) (* _impactnormal (`KismetMathLibrary.Lerp` (`self.HoverForce`) 0.0 (/ (`KismetMathLibrary.VSize` (- _location (`self.K2_GetComponentLocation`))) (`self.TraceLength`)))) (`self.K2_GetComponentLocation`) "None")
        (`PrimitiveComponent.SetLinearDamping` (`self.ParentComponent`) (`self.LinearDamping`))
        (`PrimitiveComponent.SetAngularDamping` (`self.ParentComponent`) (`self.AngularDamping`))))))

(fn `SetDebug`
  (params (bDebug :type Boolean))
  (set `self.bDebug` bDebug))